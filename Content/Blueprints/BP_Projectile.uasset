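; Grenade projectile that launches along a forward vector, explodes as a multicast event and has a short life span, with a server-started fuse timer.
; On authority, the explosion damages overlapping ThirdPersonCharacters through a GAS effect spec, passing negated DamageValue as a SetByCaller Health magnitude.
; Remote instances play the explosion particles and sound and hide the sphere.
; A simpler direct effect-application alternative remains unconnected.
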(event `self.ReceiveBeginPlay`
  (`self.SetLifeSpan` 5.0)
  (`/Engine/EditorBlueprintResources/ActorMacros.Switch Has Authority`
    (:`Authority`
      (`SceneComponent.SetVisibility` (`self.Sphere`) false false)
      (`KismetSystemLibrary.K2_SetTimerDelegate` (`|CreateDelegate` :!event `EventExplode_Multicast`) 2.0))))

(event `EventExplode_Multicast`
  (bind _returnvalue (`self.K2_GetActorLocation`))
  (bind _abilitysystemcomponent (`self.AbilitySystemComponent`))
  (`/Engine/EditorBlueprintResources/ActorMacros.Switch Has Authority`
    (:`Authority`
      (for _array_element (`PrimitiveComponent.GetOverlappingActors` (`self.OverlapSphere`) "/Game/Blueprints/ThirdPersonCharacter.ThirdPersonCharacter_C")
        ;[1 0.9627 0.4828] Option B: make gameplay spec and assign Health attribute using caller's Damage Value
        (bind _returnvalue_2 (`AbilitySystemBlueprintLibrary.AssignTagSetByCallerMagnitude` (`AbilitySystemComponent.MakeOutgoingSpec` _abilitysystemcomponent "/Game/Abilities/Effects/GE_GrenadeInstantDamage.GE_GrenadeInstantDamage_C" 0.0 (`AbilitySystemComponent.MakeEffectContext` _abilitysystemcomponent)) (struct :`TagName` "DataTag.Health") (* (`self.DamageValue`) -1.0)))
        (`AbilitySystemComponent.BP_ApplyGameplayEffectSpecToTarget` _abilitysystemcomponent _returnvalue_2 (`AbilitySystemBlueprintLibrary.GetAbilitySystemComponent` _array_element))))
    (:`Remote`
      (`GameplayStatics.SpawnEmitterAtLocation` "/Game/StarterContent/Particles/P_Explosion.P_Explosion" _returnvalue (struct) (`KismetMathLibrary.MakeVector` 5.0 5.0 5.0) true "AutoRelease")
      (`GameplayStatics.SpawnSoundAtLocation` "/Game/StarterContent/Audio/Explosion_Cue.Explosion_Cue" _returnvalue (struct) 1.0 1.0 0.0 null null)
      (`SceneComponent.SetVisibility` (`self.Sphere`) false false))))

(fn `UserConstructionScript`
  (set `MovementComponent.Velocity` (* (`self.ForwardVector`) (`KismetMathLibrary.Conv_DoubleToVector` (`ProjectileMovementComponent.InitialSpeed` (`self.ProjectileMovement`)))) (`self.ProjectileMovement`)))